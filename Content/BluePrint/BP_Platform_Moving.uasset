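; BP_Platform_Moving is a moving platform that shuttles its Cube back and forth along a Spline, starting at BeginPlay.
; A Timeline value scaled by spline length sets the Cube's world location and rotation, with pitch held at zero so only roll and yaw follow the spline.
; On each finish, a Reverse flag switches between playing forward and reversing, forming an endless ping-pong loop.
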(event `EventNormal`
  (bind _spline (`self.Spline`))
  (bind _cube (`self.Cube`))
  (bind (_returnvalue_roll _returnvalue_pitch _returnvalue_yaw) (`KismetMathLibrary.BreakRotator` (`SplineComponent.GetRotationAtDistanceAlongSpline` (`self.Spline`) 0.0 "Local")))
  (set `self.Reverse` false)
  (`SceneComponent.K2_SetRelativeRotation` (`self.Cube`) (`KismetMathLibrary.MakeRotator` _returnvalue_roll 0.0 _returnvalue_yaw) false false :!label _label)
  (bind (_direction _timer) (`Timeline|Timeline` :!label _label_2)
    (:`Update`
      (bind _returnvalue (* _timer (`SplineComponent.GetSplineLength` _spline)))
      (`SceneComponent.K2_SetWorldLocation` _cube (`SplineComponent.GetLocationAtDistanceAlongSpline` _spline _returnvalue "World") false false)
      (bind (_returnvalue_roll_2 _returnvalue_pitch_2 _returnvalue_yaw_2) (`KismetMathLibrary.BreakRotator` (`SplineComponent.GetRotationAtDistanceAlongSpline` _spline _returnvalue "World")))
      (`SceneComponent.K2_SetWorldRotation` _cube (`KismetMathLibrary.MakeRotator` _returnvalue_roll_2 0.0 _returnvalue_yaw_2) false false))
    (:`Finished`
      (if (`self.Reverse`)
        (`self.EventNormal`)
        (else
          (`self.EventReverse`))))))

(event `self.ReceiveBeginPlay`
  (goto _label))

(event `EventReverse`
  (set `self.Reverse` true)
  (goto _label_2 :!via `Reverse`))

(fn `UserConstructionScript`)