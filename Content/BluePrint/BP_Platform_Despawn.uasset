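; BP_Platform_Despawn is a platform that disappears shortly after something overlaps its Box component.
; Any overlap starts a short delay, after which the actor is flagged as destroyed, hidden and stripped of collision rather than actually destroyed.
; ResetPlateform restores the transform saved at BeginPlay, along with visibility, collision and the flag; nothing in this Blueprint calls it.
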(event `self.ReceiveBeginPlay`
  (set `self.InitialTransform` (`self.GetTransform`)))

(event `self.Box.OnComponentBeginOverlap`
  (params (OverlappedComponent :type "PrimitiveComponent Object Reference") (OtherActor :type "Actor Object Reference") (OtherComp :type "PrimitiveComponent Object Reference") (OtherBodyIndex :type Integer) (bFromSweep :type Boolean) (SweepResult :type "HitResult Structure (by ref)"))
  (`KismetSystemLibrary.Delay` 0.75)
  (set `self.IsDestroyed` true)
  (`self.SetActorHiddenInGame` true)
  (`self.SetActorEnableCollision` false))

(fn `ResetPlateform`
  (`self.K2_SetActorTransform` (`self.InitialTransform`))
  (`self.SetActorHiddenInGame` false)
  (`self.SetActorEnableCollision` true)
  (set `self.IsDestroyed` false))

(fn `UserConstructionScript`)