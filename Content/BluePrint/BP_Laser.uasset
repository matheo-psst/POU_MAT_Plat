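; BP_Laser is a moving hazard that travels along a spline and damages the third-person character.
; A timeline maps its value to spline distance, updating the Cube's location and rotation with pitch held at zero.
; On finish, the timeline alternates between play and reverse for continuous back-and-forth motion.
; Overlapping the Box writes Damage into BP_ThirdPersonCharacter's DamageTaken and calls LoseLife.
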(event `EventNormal`
  (bind _spline (`self.Spline`))
  (bind _cube (`self.Cube`))
  (bind (_returnvalue_roll _returnvalue_pitch _returnvalue_yaw) (`KismetMathLibrary.BreakRotator` (`SplineComponent.GetRotationAtDistanceAlongSpline` (`self.Spline`) 0.0 "World")))
  ; Moving/reverse
  (set `self.Reverse` false)
  (`SceneComponent.K2_SetRelativeRotation` (`self.Cube`) (`KismetMathLibrary.MakeRotator` _returnvalue_roll 0.0 _returnvalue_yaw) false false :!label _label)
  (bind (_direction _timer) (`Timeline|Timeline` :!label _label_2)
    (:`Update`
      (bind _returnvalue (* _timer (`SplineComponent.GetSplineLength` _spline)))
      (`SceneComponent.K2_SetWorldLocation` _cube (`SplineComponent.GetLocationAtDistanceAlongSpline` _spline _returnvalue "World") false false)
      (bind (_returnvalue_roll_2 _returnvalue_pitch_2 _returnvalue_yaw_2) (`KismetMathLibrary.BreakRotator` (`SplineComponent.GetRotationAtDistanceAlongSpline` _spline _returnvalue "World")))
      (`SceneComponent.K2_SetWorldRotation` _cube (`KismetMathLibrary.MakeRotator` _returnvalue_roll_2 0.0 _returnvalue_yaw_2) false false))
    (:`Finished`
      (if (`self.Reverse`)
        (`self.EventNormal`)
        (else
          (`self.EventReverse`))))))

(event `self.ReceiveBeginPlay`
  ; Moving/reverse
  (goto _label))

(event `EventReverse`
  ; Moving/reverse
  (set `self.Reverse` true)
  (goto _label_2 :!via `Reverse`))

(event `self.Box.OnComponentBeginOverlap`
  (params (OverlappedComponent :type "PrimitiveComponent Object Reference") (OtherActor :type "Actor Object Reference") (OtherComp :type "PrimitiveComponent Object Reference") (OtherBodyIndex :type Integer) (bFromSweep :type Boolean) (SweepResult :type "HitResult Structure (by ref)"))
  ; Damage
  (bind _asbp_third_person_character (cast `/Game/Characters/BP_ThirdPersonCharacter` OtherActor))
  (set `/Game/Characters/BP_ThirdPersonCharacter.DamageTaken` (`self.Damage`) _asbp_third_person_character)
  (`/Game/Characters/BP_ThirdPersonCharacter.LoseLife` _asbp_third_person_character))

(fn `UserConstructionScript`)